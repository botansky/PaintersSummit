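; Procedural track actor that builds a randomly winding, descending spline and adds spline mesh components along it.
; AddTrackData extends the data array and spline from the last point, randomizing sideways offset and a bank value that is never applied.
; DrawTrackBetweenPoints runs from construction and BeginPlay, calling AddTrackData, then setting point locations and creating meshes.
; Every mesh starts at spline point 0, and the component attach node is unconnected despite manual attachment.
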(event `self.ReceiveBeginPlay`
  (`self.DrawTrackBetweenPoints` (`self.LastDrawnIndex`) 5))

(fn `AddTrackData`
  (params (StartIndex :type Integer) (EndIndex :type Integer))
  (bind _output_position (break `/Game/Data/TrackData` (`|GetArrayItem` (`self.TrackDataArray`) (`KismetArrayLibrary.Array_LastIndex` (`self.TrackDataArray`)))))
  (bind _output (`|GetArrayItem` (`self.TrackDataArray`) (`KismetArrayLibrary.Array_LastIndex` (`self.TrackDataArray`))))
  (for _ (range StartIndex (+ (- EndIndex 2) 1))
    (`KismetArrayLibrary.Array_Add` (`self.TrackDataArray`) (make `/Game/Data/TrackData` (`KismetMathLibrary.MakeVector` (+ (.x (break `/Game/Data/TrackData` _output)) 200.0) (+ (.y (break `/Game/Data/TrackData` _output)) (`KismetMathLibrary.RandomFloatInRange` -100.0 100.0)) (- (.z (break `/Game/Data/TrackData` _output)) 100.0)) (`KismetMathLibrary.RandomFloatInRange` -5.0 5.0)))
    (`SplineComponent.AddSplinePoint` (`self.Spline`) _output_position "Local" true)))

(fn `DrawTrackBetweenPoints`
  (params (StartIndex :type Integer) (EndIndex :type Integer))
  (bind _spline (`self.Spline`))
  (bind _endindex (`self.EndIndex`))
  (bind (_location _tangent) (`SplineComponent.GetLocationAndTangentAtSplinePoint` _spline 0 "Local"))
  (`self.AddTrackData` StartIndex EndIndex)
  (for _index (range (`self.StartIndex`) (+ _endindex 1))
    (bind _output_position (break `/Game/Data/TrackData` (`|GetArrayItem` (`self.TrackDataArray`) _index)))
    (`SplineComponent.SetLocationAtSplinePoint` (`self.Spline`) _index _output_position "Local" true)
    (bind _returnvalue (+ _index 1))
    (bind _output_position_2 (break `/Game/Data/TrackData` (`|GetArrayItem` (`self.TrackDataArray`) _returnvalue)))
    (`SplineComponent.SetLocationAtSplinePoint` (`self.Spline`) _returnvalue _output_position_2 "Local" true)
    (bind _returnvalue_2 (`AddComponent|NODE_AddSplineMeshComponent-0` :`bManualAttachment` true))
    (bind (_location_2 _tangent_2) (`SplineComponent.GetLocationAndTangentAtSplinePoint` _spline _returnvalue "Local"))
    (`SplineMeshComponent.SetStartAndEnd` _returnvalue_2 _location _tangent _location_2 _tangent_2 true))
  (set `self.LastDrawnIndex` _endindex))

(fn `UserConstructionScript`
  (set `self.StartIndex` 0)
  (set `self.EndIndex` (- (`SplineComponent.GetNumberOfSplinePoints` (`self.Spline`)) 2))
  (`self.DrawTrackBetweenPoints` (`self.StartIndex`) (`self.EndIndex`)))
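; Track generator actor that builds a track from spline mesh components along a spline, with optional left and right banks and switchable collision.
; UpdateTrack loops over the spline point count cached at construction, shaping each segment's roll, width and thickness from TrackDataArray.
; BeginPlay repeatedly appends a descending point with random sideways offset and roll, then calls UpdateTrack.
; UpdateTrack adds new meshes without clearing earlier ones or refreshing that count.
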(event `self.ReceiveBeginPlay`
  (for _ (range 6)
    (`self.AddSplinePoint`)
    (`self.UpdateTrack`)))

(fn `AddSplinePoint`
  (locals (NewPosition :type "Vector Structure"))
  (bind _output (`|GetArrayItem` (`self.TrackDataArray`) (`KismetArrayLibrary.Array_LastIndex` (`self.TrackDataArray`))))
  (set `local.NewPosition` (`KismetMathLibrary.MakeVector` (+ (.x (break `/Game/Data/TrackData` _output)) 200.0) (+ (.y (break `/Game/Data/TrackData` _output)) (`KismetMathLibrary.RandomFloatInRange` -100.0 100.0)) (- (.z (break `/Game/Data/TrackData` _output)) 100.0)))
  (`KismetArrayLibrary.Array_Add` (`self.TrackDataArray`) (make `/Game/Data/TrackData` (`local.NewPosition`) (`KismetMathLibrary.RandomFloatInRange` -5.0 5.0)))
  (`SplineComponent.AddPoint` (`self.Spline`) (make `SplinePoint` 0.0 (`local.NewPosition`)) true))

(fn `BuildTrackElement`
  (params (Index :type Integer) (TrackMeshElement :type "StaticMesh Object Reference"))
  (locals (Local_CurrentIndex :type Integer) (Local_NextIndex :type Integer :default 0) (Local_TrackElementMesh :type "StaticMesh Object Reference") (Local_StartPosition :type "Vector Structure") (Local_StartTangent :type "Vector Structure") (Local_EndPosition :type "Vector Structure") (Local_EndTangent :type "Vector Structure") (Local_CurrentSplineMesh :type "SplineMeshComponent Object Reference") (Local_StartRoll :type "Float (double-precision)") (Local_StartScale :type "Vector2D Structure") (Local_EndRoll :type "Float (double-precision)") (Local_EndScale :type "Vector2D Structure"))
  (bind (_output_position _output_trackbank _output_trackwidth _output_trackthickness) (break `/Game/Data/TrackData` (`|GetArrayItem` (`self.TrackDataArray`) (`local.Local_NextIndex`))))
  (bind (_output_position_2 _output_trackbank_2 _output_trackwidth_2 _output_trackthickness_2) (break `/Game/Data/TrackData` (`|GetArrayItem` (`self.TrackDataArray`) (`local.Local_CurrentIndex`))))
  (bind _output_position_3 (break `/Game/Data/TrackData` (`|GetArrayItem` (`self.TrackDataArray`) (`local.Local_NextIndex`))))
  (set `local.Local_CurrentIndex` Index)
  (set `local.Local_NextIndex` (mod (+ Index 1) (`self.SplinePtCount`)))
  (set `local.Local_TrackElementMesh` TrackMeshElement)
  (`|ExecutionSequence`
    (:`then_0`
      (set `local.Local_StartPosition` (`SplineComponent.GetLocationAndTangentAtSplinePoint` (`self.Spline`) (`local.Local_CurrentIndex`) "Local"))
      (set `local.Local_EndPosition` _output_position_3)
      (set `local.Local_StartRoll` _output_trackbank_2)
      (set `local.Local_StartScale` (`KismetMathLibrary.MakeVector2D` _output_trackwidth_2 _output_trackthickness_2))
      (set `local.Local_EndRoll` _output_trackbank)
      (set `local.Local_EndScale` (`KismetMathLibrary.MakeVector2D` _output_trackwidth _output_trackthickness)))
    (:`then_1`
      (bind _returnvalue (`AddComponent|NODE_AddSplineMeshComponent-0`))
      (set `local.Local_CurrentSplineMesh` _returnvalue)
      (`StaticMeshComponent.SetStaticMesh` (`local.Local_CurrentSplineMesh`) (`local.Local_TrackElementMesh`))
      (`SplineMeshComponent.SetStartAndEnd` (`local.Local_CurrentSplineMesh`) (`local.Local_StartPosition`) (0.0 0.0 0.0) (`local.Local_EndPosition`) (0.0 0.0 0.0) false)
      (`SplineMeshComponent.SetStartRoll` (`local.Local_CurrentSplineMesh`) (`local.Local_StartRoll`) false)
      (`SplineMeshComponent.SetEndRoll` (`local.Local_CurrentSplineMesh`) (`local.Local_EndRoll`) true)
      (`SplineMeshComponent.SetStartScale` (`local.Local_CurrentSplineMesh`) (`local.Local_StartScale`) true)
      (`SplineMeshComponent.SetEndScale` (`local.Local_CurrentSplineMesh`) (`local.Local_EndScale`) true)
      (`PrimitiveComponent.SetCollisionEnabled` (`local.Local_CurrentSplineMesh`) (select `bool` (`self.Collisions`) :`false` "NoCollision" :`true` "QueryAndPhysics" :!type "ECollisionEnabled Enum")))))

(fn `UpdateTrack`
  (bind (_output_position _output_trackbank _output_trackwidth _output_trackthickness _output_rbank _output_lbank) (break `/Game/Data/TrackData` (`|GetArrayItem` (`self.TrackDataArray`) (`self.CurrentIndex`))))
  (for _index (range (`self.StartIndex`) (+ (- (`self.SplinePtCount`) (`KismetMathLibrary.SelectInt` 1 2 (`self.ClosedTrack`))) 1))
    (set `self.CurrentIndex` _index)
    (set `self.DrawRBank` _output_rbank)
    (set `self.DrawLBank` _output_lbank)
    (`|ExecutionSequence`
      (:`then_0`
        (`self.BuildTrackElement` (`self.CurrentIndex`) (`self.TrackMesh`)))
      (:`then_1`
        (if (`self.DrawLBank`)
          (`self.BuildTrackElement` (`self.CurrentIndex`) (`self.LBankMesh`))))
      (:`then_2`
        (if (`self.DrawRBank`)
          (`self.BuildTrackElement` (`self.CurrentIndex`) (`self.RBankMesh`)))))))

(fn `UserConstructionScript`
  (set `self.SplinePtCount` (`SplineComponent.GetNumberOfSplinePoints` (`self.Spline`)))
  (`self.UpdateTrack`))